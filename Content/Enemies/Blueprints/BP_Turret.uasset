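; Enemy turret that turns toward the player character when pawn sensing spots it and fires bullets with a sound from its arrow.
; The first sighting fires after a brief random delay, while a fixed Delay paces shots as sightings continue.
; Projectile hits and general damage reduce health, shown on a widget bar hidden at full health.
; At zero health it optionally spawns a loot drop, then destroys itself.
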(event OnSeePawn(PawnSensing)
  (params (Pawn :type Pawn%20Object%20Reference))
  (bind _returnvalue (Transformation|GetActorLocation Pawn))
  (bind _returnvalue_2 (Transformation|GetActorLocation))
  (bind _arrow (Variables|Default|GetArrow))
  (Utilities|Casting|CastToBP_FirstPersonCharacter Pawn)
  (Transformation|SetActorRotation (Math|Rotator|FindLookatRotation (Math|Vector|MakeVector (.x _returnvalue_2) (.y _returnvalue_2) 0.0) (Math|Vector|MakeVector (.x _returnvalue) (.y _returnvalue) 0.0)))
  (Utilities|FlowControl|Delay (Math|Random|RandomFloatinRange 0.0 0.2))
  (Utilities|FlowControl|Sequence
    (:then_0
      (Utilities|FlowControl|DoOnce false
        (:Completed
          _)))
    (:then_1
      (Utilities|FlowControl|Delay 3.5)))
  (Game|SpawnActorfromClass "/Game/Enemies/Blueprints/BP_TurretBullet.BP_TurretBullet_C" (Transformation|GetWorldTransform _arrow) "Undefined" "OverrideRootScale" 0 0)
  (Audio|PlaySoundatLocation "/Game/FPWeapon/Audio/FirstPersonTemplateWeaponFire02.FirstPersonTemplateWeaponFire02" (Variables|/Script/Engine.SceneComponent|GetRelativeLocation _arrow) "0, 0, 0" 1.0 1.0 0.0 0 0 0 0) ; Play firing sound
)

(event Custom|IsDead?
  ;[1 1 1] Remove ennemy if no more health
  (if (<= (Variables|Default|GetHealth) 0)
    (if (Variables|Default|GetMakeDrop)
      (CallFunction|DropLoot))
    (Actor|DestroyActor)))

(event Custom|Drop%20Loot
  ;[1 1 1] Drop loot
  (Game|SpawnActorfromClass (Variables|Default|GetObjectDrop) (Transformation|GetWorldTransform (Variables|Default|GetArrow)) "Undefined" "OverrideRootScale" 0 0))

(event EventTick
  (params (DeltaSeconds :type Float%20%28single-precision%29))
  (bind _aswbp_health_bar (Utilities|Casting|CastToWBP_HealthBar (UserInterface|GetWidget (Variables|Default|GetHealth%20Bar%20Widget))))
  (Progress|SetPercent (Variables|/Game/Enemies/Blueprints/WBP_HealthBar.WBP_HealthBar_C|GetHealthBar _aswbp_health_bar) (/ (Math|Conversions|ToFloat(Integer) (Variables|Default|GetHealth)) (Math|Conversions|ToFloat(Integer) (Variables|Default|GetMaxHealth))))
  (Variables|/Game/LevelPrototyping/Blueprints/BP_RotateTowardsPlayer.BP_RotateTowardsPlayer_C|SetTarget (Variables|Default|GetBP_RotateTowardsPlayer) (Variables|Default|GetHealth%20Bar%20Widget))
  ;[1 1 1] Do not bloat if health is full
  (Rendering|SetVisibility (Variables|Default|GetHealth%20Bar%20Widget) (not (== (Variables|Default|GetHealth) (Variables|Default|GetMaxHealth))) false))

(event EventBeginPlay
  (Variables|Default|SetMaxHealth (Variables|Default|GetHealth)))

(event Collision|EventHit
  (params (MyComp :type Primitive%20Component%20Object%20Reference) (Other :type Actor%20Object%20Reference) (OtherComp :type Primitive%20Component%20Object%20Reference) (bSelfMoved :type Boolean) (HitLocation :type Vector :default "0, 0, 0") (HitNormal :type Vector :default "0, 0, 0") (NormalImpulse :type Vector :default "0, 0, 0") (Hit :type Hit%20Result%20Structure%20%28by%20ref%29))
  (Utilities|Casting|CastToBP_FirstPersonProjectile Other)
  (Variables|Default|SetHealth (- (Variables|Default|GetHealth) 1))
  (CallFunction|IsDead?))

(event Game|Damage|EventAnyDamage
  (params (Damage :type Float%20%28single-precision%29) (DamageType :type Damage%20Type%20Object%20Reference) (InstigatedBy :type Controller%20Object%20Reference) (DamageCauser :type Actor%20Object%20Reference))
  ;[1 1 1] Explosion range damage
  (Variables|Default|SetHealth (Math|Float|Truncate (- (Variables|Default|GetHealth) Damage)))
  (CallFunction|IsDead?))

(fn ConstructionScript)